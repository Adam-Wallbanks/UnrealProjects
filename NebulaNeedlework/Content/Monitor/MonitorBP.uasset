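; Monitor Blueprint that shows step-by-step videos for a syringe procedure through a shared media player.
; Five seconds after BeginPlay, it opens the first syringe draw-up video.
; Three functions switch the media player to the clips for after the syringe-vial connection, after connecting to the man, and mission completion after the bin.
; None of these functions are called within this Blueprint.
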(event EventBeginPlay
  (Utilities|FlowControl|Delay 5.0)
  (Media|MediaPlayer|OpenSource (Variables|Default|GetmediaplayerMonitor) "/Game/Movies/First_Syringe_Draw_Up_Vid.First_Syringe_Draw_Up_Vid"))

(fn ConstructionScript)

(fn PlayAfterSyringeConnect
  (Media|MediaPlayer|OpenSource (Variables|Default|GetmediaplayerMonitor) "/Game/Movies/After_Syringe_Vial_Connect_Vid_-_Made_With_Clipchamp.After_Syringe_Vial_Connect_Vid_-_Made_With_Clipchamp"))

(fn PlayAfterManConnect
  (Media|MediaPlayer|OpenSource (Variables|Default|GetmediaplayerMonitor) "/Game/Movies/Before_Garbage_Chute_After_Connect_To_Man_-_Made_With_Clipchamp.Before_Garbage_Chute_After_Connect_To_Man_-_Made_With_Clipchamp"))

(fn FinalPlay
  (Media|MediaPlayer|OpenSource (Variables|Default|GetmediaplayerMonitor) "/Game/Movies/Mission_Complete_Vid_For_After_The_Bin_-_Made_With_Clipchamp.Mission_Complete_Vid_For_After_The_Bin_-_Made_With_Clipchamp"))