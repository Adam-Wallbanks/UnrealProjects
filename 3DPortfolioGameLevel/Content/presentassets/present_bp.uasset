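; Interactable present actor that turns into a toy car when the player presses Interact nearby.
; Overlap of a trigger component by the FirstPersonCharacter opens a gate, and leaving closes it.
; The actor enables its own input on BeginPlay; an Interact press passing the open gate swaps the Present1 static mesh to the Toycar mesh.
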(event OnComponentBeginOverlap(2)
  (params (OverlappedComponent :type Primitive%20Component%20Object%20Reference) (OtherActor :type Actor%20Object%20Reference) (OtherComp :type Primitive%20Component%20Object%20Reference) (OtherBodyIndex :type Integer) (bFromSweep :type Boolean) (SweepResult :type Hit%20Result%20Structure%20%28by%20ref%29))
  (Utilities|Casting|CastToFirstPersonCharacter OtherActor)
  (Utilities|FlowControl|Gate true) ; enters at Open
)

(event OnComponentEndOverlap(2)
  (params (OverlappedComponent :type Primitive%20Component%20Object%20Reference) (OtherActor :type Actor%20Object%20Reference) (OtherComp :type Primitive%20Component%20Object%20Reference) (OtherBodyIndex :type Integer))
  (Utilities|Casting|CastToFirstPersonCharacter OtherActor)
  (Utilities|FlowControl|Gate true) ; enters at Close
)

(event EventBeginPlay
  (Variables|Default|Setpresent1 (Variables|Default|Getpresent1))
  (Input|EnableInput (Game|GetPlayerController 0)))

(event Input|ActionEvents|InputActionInteract
  (params (Key :type Key%20Structure))
  (:Pressed
    (Utilities|FlowControl|Gate true
      (:Exit
        (Components|StaticMesh|SetStaticMesh (Variables|Default|Getpresent1) "/Game/Toycarassets/toycar.toycar")))))

(fn ConstructionScript)